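; BP_TargetBPActor is a target actor that moves along the vertical axis and carries a configurable text and image widget.
; On BeginPlay it stores its starting positions, then a timeline drives its height as an offset from the start, scaled by MoveAmplitude.
; SetWidgetContent sets widget visibility, passes text, color, texture and index to WD_Text, and shifts the widget by WidgetOffset.
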(event EventBeginPlay
  (Variables|InitialValue|SetInitialLocation (Transformation|GetActorLocation))
  (Variables|InitialValue|SetInitialWidgetLocation (Variables|/Script/Engine.SceneComponent|GetRelativeLocation (Variables|Default|GetWidget)))
  (CallFunction|SetWidgetContent)
  (bind _l5s0_1_0 (Timeline|Timeline PlayFromStart)
    (:Update
      (Transformation|SetActorLocation (+ (Variables|InitialValue|GetInitialLocation) (Math|Vector|MakeVector 0.0 0.0 (* _l5s0_1_0 (Variables|User|Movement|GetMoveAmplitude)))) false false))))

(event Collision|EventActorBeginOverlap
  (params (OtherActor :type Actor%20Object%20Reference)))

(fn ConstructionScript)

(fn SetWidgetContent
  (bind _widget (Variables|Default|GetWidget))
  (Rendering|SetVisibility _widget (Variables|User|Widget|GetbShowWidget) false)
  (bind _aswd_text (Utilities|Casting|CastToWD_Text (UserInterface|GetUserWidgetObject _widget)))
  (Default|ChangeWidgetInfo _aswd_text (Variables|User|Widget|GetWidgetText) (Variables|User|Widget|GetTextColor) (Variables|User|Widget|GetWidgetTexture) (Variables|Default|GetIndex))
  (Transformation|SetRelativeLocation _widget (+ (Variables|InitialValue|GetInitialWidgetLocation) (Variables|User|Widget|GetWidgetOffset)) false false))